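; BP_Hide is a hiding spot actor that lets the player's dog hide and unhide with the Hide input action.
; Box overlap with BP_Dog caches the dog, enables input and opens a gate, while leaving disables input and closes it.
; The gated press toggles the dog's hide state; hiding also blends the view to this actor, then re-enables input and reopens the gate after a short delay.
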(event `InputAction|Hide`
  (params (Key :type "Key Structure"))
  (bind _as_bp_dog (`self.As BP Dog`))
  (:`Pressed`
    (`/Engine/EditorBlueprintResources/StandardMacros.Gate` true :!label _label
      (:`Exit`
        (if (`/Game/ThirdPerson/Blueprints/BP_Dog.IsHiding` _as_bp_dog)
          (`/Game/ThirdPerson/Blueprints/BP_Dog.Unhide` _as_bp_dog)
          (else
            (`/Game/ThirdPerson/Blueprints/BP_Dog.Hide` _as_bp_dog)
            (`|ExecutionSequence`
              (:`then_0`
                (`PlayerController.SetViewTargetWithBlend` (`GameplayStatics.GetPlayerController` 0) self 0.5 "VTBlend_Linear" 0.0 false))
              (:`then_1`
                (`KismetSystemLibrary.Delay` 0.2)
                (`self.EnableInput` (`GameplayStatics.GetPlayerController` 0) null :!label _label_2)
                (goto _label :!via `Open`)))))))))

(event `self.Box.OnComponentBeginOverlap`
  (params (OverlappedComponent :type "PrimitiveComponent Object Reference") (OtherActor :type "Actor Object Reference") (OtherComp :type "PrimitiveComponent Object Reference") (OtherBodyIndex :type Integer) (bFromSweep :type Boolean) (SweepResult :type "HitResult Structure (by ref)"))
  (bind _asbp_dog (cast `/Game/ThirdPerson/Blueprints/BP_Dog` OtherActor))
  (set `self.As BP Dog` _asbp_dog)
  (goto _label_2))

(event `self.Box.OnComponentEndOverlap`
  (params (OverlappedComponent :type "PrimitiveComponent Object Reference") (OtherActor :type "Actor Object Reference") (OtherComp :type "PrimitiveComponent Object Reference") (OtherBodyIndex :type Integer))
  (cast `/Game/ThirdPerson/Blueprints/BP_Dog` OtherActor)
  (`self.DisableInput` (`GameplayStatics.GetPlayerController` 0) null)
  (goto _label :!via `Close`))

(fn `UserConstructionScript`)